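; BP_Nest is a spawner actor that creates a configurable actor at its own transform when SpawnActor is called, unless a previous spawn is still cooling down.
; It hands the new actor a target, a reference to itself, and an AI controller class with behavior tree through three chained interface casts.
; A successful setup plays an optional sound and starts the cooldown; a failed cast prints an error and releases the lock immediately.
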(event `/Game/Turtles/Blueprints/Interfaces/BPI_Spawn.SpawnActor`
  (bind _sound (`self.Sound`))
  ;[1 1 1] Spawning process
  (if (`self.SpawnProcess`)
    (`KismetSystemLibrary.PrintString` "Spawning on cooldown" true true (struct :`R` 0.985119 :`G` 1.0 :`A` 1.0))
    (else
      (set `self.SpawnProcess` true)
      (bind _returnvalue (`|SpawnActorFromClass` (`self.ActorToSpawn`) (`self.GetTransform` self) "Undefined" "OverrideRootScale" null null))
      ;[1 1 1] Has Target Interface
      (bind _asbpi_has_target (cast `/Game/Turtles/Blueprints/Interfaces/BPI_HasTarget` _returnvalue)
        (:`then`
          (`/Game/Turtles/Blueprints/Interfaces/BPI_HasTarget.SetTarget` _asbpi_has_target (`self.TargetActor`))
          ;[1 1 1] Has Nest Interface
          (bind _asbpi_has_nest (cast `/Game/Turtles/Blueprints/Interfaces/BPI_HasNest` _returnvalue)
            (:`then`
              (`/Game/Turtles/Blueprints/Interfaces/BPI_HasNest.SetNest` _asbpi_has_nest self)
              ;[1 1 1] Has BehaviorTree Interface
              (bind _asbpi_has_ai (cast `/Game/Turtles/Blueprints/Interfaces/BPI_HasAI` _returnvalue)
                (:`then`
                  (`/Game/Turtles/Blueprints/Interfaces/BPI_HasAI.SetAIData` _asbpi_has_ai (`self.AIControllerClass`) (`self.BehaviorTree`))
                  ;[1 1 1] Play Sound Effect
                  (`/Engine/EditorBlueprintResources/StandardMacros.IsValid` _sound
                    (:`Is Valid`
                      (`GameplayStatics.PlaySoundAtLocation` _sound (`self.K2_GetActorLocation` self) (struct) 1.0 1.0 0.0 null null null))
                    (:`Is Not Valid`
                      _))
                  ;[1 1 1] Cooldown
                  (`KismetSystemLibrary.Delay` (`self.Cooldown`))
                  (set `self.SpawnProcess` false))
                (:`CastFailed`
                  (`KismetSystemLibrary.PrintString` "Can't cast object to BPI_HasAI" true true (struct :`R` 1.0 :`B` 0.039766 :`A` 1.0))
                  (set `self.SpawnProcess` false))))
            (:`CastFailed`
              (`KismetSystemLibrary.PrintString` "Can't cast object to BPI_HasNest" true true (struct :`R` 1.0 :`B` 0.008869 :`A` 1.0))
              (set `self.SpawnProcess` false))))
        (:`CastFailed`
          (`KismetSystemLibrary.PrintString` "Can't cast object to BPI_HasTarget" true true (struct :`R` 1.0 :`B` 0.008869 :`A` 1.0))
          (set `self.SpawnProcess` false))))))

(fn `UserConstructionScript`)